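; Billiards cue actor that attaches to the cue ball and handles aiming, shooting, Tab camera toggling and R restart.
; Axis input rotates the ball to aim with clamped roll, or with right mouse held slides the cue within a clamped strike offset.
; Shoot disables further shots and applies impulse and torque to the ball, derived from cue offset and ball rotation.
; Switching to the top camera blocks shooting; returning to the cue view re-enables it.
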(event EventBeginPlay
  (Utilities|FlowControl|Delay 0.2)
  (Transformation|AttachActorToActor (Variables|Default|GetCueBall) "None" "KeepRelative" "KeepRelative" "KeepRelative" true)
  (Transformation|SetActorRelativeTransform (Math|Transform|MakeTransform "0.000000,-775.000000,0.000000" "0.000000,-180.000000,0.000000") false false))

(event EventTick
  (params (DeltaSeconds :type Float%20%28single-precision%29))
  (bind _returnvalue (Class|Actor|GetInputAxisKeyValue))
  (bind _returnvalue_2 (Class|Actor|GetInputAxisKeyValue))
  (bind _cueball (Variables|Default|GetCueBall))
  (bind _defaultsceneroot (Variables|Default|GetDefaultSceneRoot))
  (bind _offsetclamp (Variables|Default|GetoffsetClamp))
  (bind _returnvalue_3 (* -1 _returnvalue_2))
  (bind _returnvalue_4 (Transformation|GetActorRotation _cueball))
  (bind _relativelocation (Variables|/Script/Engine.SceneComponent|GetRelativeLocation _defaultsceneroot))
  (bind _returnvalue_5 (Math|Vector|MakeVector _returnvalue_3 0.0 _returnvalue))
  (bind (_roll _pitch _yaw) (Math|Rotator|BreakRotator _returnvalue_4))
  (bind _returnvalue_6 (+ _relativelocation _returnvalue_5))
  (bind (_x _y _z) (Math|Vector|BreakVector _returnvalue_6))
  (bind _returnvalue_7 (Math|Vector|MakeVector _x 0.0 _z))
  (bind _returnvalue_8 (Math|Vector|ClampVectorSize _returnvalue_7 0.0 _offsetclamp))
  (bind (_x_2 _y_2 _z_2) (Math|Vector|BreakVector _returnvalue_8))
  (if (or (!= (Class|Actor|GetInputAxisKeyValue) 0.0) (!= (Class|Actor|GetInputAxisKeyValue) 0.0))
    (if (Variables|Default|GetcanShoot)
      (if (Game|Player|IsInputKeyDown (Game|GetPlayerController 0) "RightMouseButton")
        (Transformation|SetActorRelativeLocation (Math|Vector|MakeVector _x_2 _y _z_2))
        (else
          (Transformation|AddActorLocalRotation (Variables|Default|GetCueBall) (Math|Rotator|MakeRotator (Class|Actor|GetInputAxisKeyValue) 0.0 (* -1 (Class|Actor|GetInputAxisKeyValue))) false false)
          (Transformation|SetActorRotation (Variables|Default|GetCueBall) (Math|Rotator|MakeRotator (Math|Float|Clamp(Float) _roll 5.0 2e+01) 0.0 _yaw)))))))

(event Input|ActionEvents|InputActionShoot
  (params (Key :type Key%20Structure))
  (bind _cueball (Variables|Default|GetCueBall))
  (bind _defaultsceneroot (Variables|Default|GetDefaultSceneRoot))
  (bind _defaultsceneroot_2 (Variables|Default|GetDefaultSceneRoot))
  (bind _cueball_2 (Variables|Default|GetCueBall))
  (bind _cueball_3 (Variables|Default|GetCueBall))
  (bind _returnvalue (Transformation|GetActorRotation _cueball))
  (bind _returnvalue_2 (Transformation|GetActorRotation _cueball_2))
  (bind _relativelocation (Variables|/Script/Engine.SceneComponent|GetRelativeLocation _defaultsceneroot))
  (bind _relativelocation_2 (Variables|/Script/Engine.SceneComponent|GetRelativeLocation _defaultsceneroot_2))
  (bind _sphere (Variables|/Game/Blueprints/BP_White_BilliardBall.BP_White_BilliardBall_C|GetSphere _cueball_3))
  (bind _returnvalue_3 (Math|Vector|RotateVector _relativelocation_2 _returnvalue_2))
  (bind (_x _y _z) (Math|Vector|BreakVector _relativelocation))
  (bind _yaw (Math|Rotator|BreakRotator _returnvalue))
  (bind _returnvalue_4 (Math|Vector|MakeVector _x 0.0 _z))
  (:Pressed
    (if (Variables|Default|GetcanShoot)
      (Variables|Default|SetcanShoot false)
      (Physics|AddImpulse _sphere (* (* (Math|Vector|Normalize _returnvalue_3) (* (- 1.0 (/ (Math|Vector|VectorLength _returnvalue_4) (Variables|Default|GetoffsetClamp))) (Math|Vector|VectorLength (* (CallFunction|SubtractVectorfromFloat (Variables|Default|GetoffsetClamp) (CallFunction|Absolute(Vector) (Math|Vector|RotateVector _returnvalue_4 _returnvalue))) (- (CallFunction|GetIdentityVector) (CallFunction|Absolute(Vector) (Math|Vector|MakeVector (Math|Trig|Sin(Degrees) _yaw) (Math|Trig|Cos(Degrees) _yaw) 0.0))))))) (Variables|Default|Getforce)) "None" false)
      (Class|PrimitiveComponent|AddTorqueinDegrees _sphere (* (Math|Vector|RotateVector (Math|Vector|Normalize (* (- (Variables|/Script/Engine.SceneComponent|GetRelativeLocation (Variables|Default|GetCueDirectionObject)) _returnvalue_3) (CallFunction|SubtractVectorfromFloat (Variables|Default|GetoffsetClamp) (CallFunction|Absolute(Vector) (Math|Vector|MakeVector _x (Variables|Default|GetoffsetClamp) _z))))) (Transformation|GetActorRotation (Variables|Default|GetCueBall))) (Variables|Default|Getforce)) "None" false))))

(event Input|KeyboardEvents|Tab
  (params (Key :type Key%20Structure))
  (:Pressed
    (Utilities|FlowControl|FlipFlop
      (:A
        (Variables|Default|SetcanShoot false)
        (Game|Player|SetViewTargetwithBlend (Game|GetPlayerController 0) (Variables|Default|GetTopCamera) 0.0 "VTBlend_Linear" 0.0 false))
      (:B
        (Variables|Default|SetcanShoot true)
        (Game|Player|SetViewTargetwithBlend (Game|GetPlayerController 0) self 0.0 "VTBlend_Linear" 0.0 false)))))

(event Input|KeyboardEvents|R
  (params (Key :type Key%20Structure))
  (:Pressed
    (bind _asbilliards_game_mode (Utilities|Casting|CastToBilliardsGameMode (Game|GetGameMode)))
    (Class|GameMode|RestartGame _asbilliards_game_mode)))

(fn ConstructionScript)