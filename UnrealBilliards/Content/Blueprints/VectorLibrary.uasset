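; VectorLibrary is a small set of vector math helper functions.
; It provides a component-wise absolute value and a float-minus-vector operation that spreads the float across all three axes before subtracting.
; GetIdentityVector returns a vector of all ones, the multiplicative identity, rather than a zero vector.
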(fn Absolute(Vector)
  (params (Vector :type Vector))
  (bind (_x _y _z) (Math|Vector|BreakVector Vector))
  (return (Math|Vector|MakeVector (Math|Float|Absolute(Float) _x) (Math|Float|Absolute(Float) _y) (Math|Float|Absolute(Float) _z))))

(fn SubtractVectorfromFloat
  (params (float :type Float%20%28single-precision%29) (Vector :type Vector))
  (return (- (Math|Vector|MakeVector float float float) Vector)))

(fn GetIdentityVector
  (return (Math|Vector|MakeVector 1.0 1.0 1.0)))